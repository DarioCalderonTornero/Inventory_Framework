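; BP_PickUpItem is a world pickup that adds its item to the inventory of the actor that overlaps it.
; On overlap, it looks for an InventoryManagerComponent on the other actor, passes ItemName to AddItem, then destroys itself.
; The construction script switches on ItemName to pick the static mesh for Bread, Wood or Potion, so one Blueprint covers each item type.
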(event Collision|EventActorBeginOverlap
  (params (OtherActor :type Actor%20Object%20Reference))
  (bind _returnvalue (Actor|GetComponentbyClass OtherActor "/Game/InventorySystem/InventoryManagerComponent.InventoryManagerComponent_C"))
  (Utilities|IsValid _returnvalue
    (:Is%20Valid
      (Default|AddItem _returnvalue (Variables|Default|GetItemName))
      (Actor|DestroyActor))))

(fn ConstructionScript
  (switch string (Variables|Default|GetItemName)
    (:Bread
      (Components|StaticMesh|SetStaticMesh (Variables|Default|GetStaticMesh) "/Game/LevelPrototyping/Meshes/SM_ChamferCube.SM_ChamferCube"))
    (:Wood
      (Components|StaticMesh|SetStaticMesh (Variables|Default|GetStaticMesh) "/Game/LevelPrototyping/Interactable/Target/Assets/SM_TargetBaseMesh.SM_TargetBaseMesh"))
    (:Potion
      (Components|StaticMesh|SetStaticMesh (Variables|Default|GetStaticMesh) "/Game/LevelPrototyping/Interactable/JumpPad/Assets/Meshes/SM_CircularGlow.SM_CircularGlow"))))