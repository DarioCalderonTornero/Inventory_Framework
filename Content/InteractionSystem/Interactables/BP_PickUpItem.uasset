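; Interactable world pickup that gives its inventory item to whoever interacts with it.
; The construction script sets the static mesh from the WorldRepresentation fragment of the item's definition, so the actor looks like the item it holds.
; On Interact it prints a debug message, and if the interactor has an InventoryManagerComponent it adds the item, plays a sound and destroys itself.
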(event EventInteract
  (params (Interactor :type Actor%20Object%20Reference))
  (bind _returnvalue (Actor|GetComponentbyClass Interactor "/Game/InventorySystem/InventoryManagerComponent.InventoryManagerComponent_C"))
  (Development|PrintString (Utilities|String|ToString(Text) (Utilities|Text|FormatText "Added{itemName} to the inventory of {ActorName}" (Utilities|GetDisplayName self) (Utilities|GetDisplayName Interactor))))
  (Utilities|IsValid _returnvalue
    (:Is%20Valid
      (Default|AddItem _returnvalue (Variables|Default|GetInventoryItem))
      (Audio|PlaySound2D "/Game/InventorySystem/Sounds/Drop_Item_From_ContentBrowser.Drop_Item_From_ContentBrowser" 1.0 1.0 0.0 0 0)
      (Actor|DestroyActor))))

(fn ConstructionScript
  (bind _inventoryitem (Variables|Default|GetInventoryItem))
  (bind _returnvalue (Class|ItemDefinition|FindFragmentbyClass (.itemdefinition _inventoryitem) "/Script/Inventory_Framework.InventoryItemFragment_WorldRepresentation"))
  (Utilities|IsValid _returnvalue
    (:Is%20Valid
      (Components|StaticMesh|SetStaticMesh (Variables|Default|GetStaticMesh) (Variables|/Script/Inventory_Framework.InventoryItemFragment_WorldRepresentation|GetItemMesh _returnvalue)))))

(fn GetInteractionType
  (return (Variables|Default|GetInteractionType)))